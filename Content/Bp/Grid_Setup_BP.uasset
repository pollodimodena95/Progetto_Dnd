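; Grid setup actor that spawns a flat GridX by GridY grid of GridBase_BP actors on BeginPlay.
; Nested loops place each cell at GridSize spacing relative to the actor's location, storing it in GridBaseArray.
; The offset subtracts the full grid extent (divisor of 1), so the last cell sits on the actor and the rest extend toward negative X and Y.
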(event `self.ReceiveBeginPlay`
  (bind _grid_x (`self.Grid X`))
  (bind _grid_y (`self.Grid Y`))
  (bind _grid_size (`self.Grid Size`))
  (bind _grid_size_2 (`self.Grid Size`))
  (for _index (range 1 (+ _grid_x 1))
    (for _index_2 (range 1 (+ _grid_y 1))
      (bind _returnvalue (`|SpawnActorFromClass` "/Game/Bp/GridBase_BP.GridBase_BP_C" (`KismetMathLibrary.MakeTransform` (+ (`KismetMathLibrary.MakeVector` (`KismetMathLibrary.Conv_IntToDouble` (- (* _index _grid_size_2) (/ (* _grid_x _grid_size) 1))) (`KismetMathLibrary.Conv_IntToDouble` (- (* _index_2 _grid_size_2) (/ (* _grid_y _grid_size) 1)))) (`self.K2_GetActorLocation`))) "AlwaysSpawn" "OverrideRootScale" null null))
      (`KismetArrayLibrary.Array_Add` (`self.Grid Base Array`) _returnvalue))))

(fn `UserConstructionScript`)